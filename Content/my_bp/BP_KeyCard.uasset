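; BP_KeyCard is a keycard pickup that activates a referenced card reader when the player presses F while overlapping it.
; It polls the F key on player controller 0 every Tick and checks overlap with the player pawn at that moment.
; A successful press calls Activate on CardReaderRef and destroys the keycard.
; Debug strings log initialization, key presses and out-of-range failures.
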(event EventBeginPlay
  (Development|PrintString "KEYCARD_INIT" false)
  (Input|EnableInput self (Game|GetPlayerController 0)))

(event Collision|EventActorBeginOverlap
  (params (OtherActor :type Actor%20Object%20Reference)))

(event EventTick
  (params (DeltaSeconds :type Float%20%28single-precision%29))
  (bind _self self)
  (if (Game|Player|WasInputKeyJustPressed (Game|GetPlayerController 0) "F")
    (Development|PrintString "F_PRESSED_ON_KEYCARD" false)
    (if (Collision|IsOverlappingActor _self (Game|Player|GetPlayerPawn 0) :!class /Script/Engine.Actor)
      (Default|Activate (Variables|Default|GetCardReaderRef))
      (Actor|DestroyActor _self)
      (else
        (Development|PrintString "KEYCARD_FAIL_NOT_IN_RANGE" false)))))

(fn ConstructionScript)