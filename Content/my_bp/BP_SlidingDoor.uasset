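; Sliding door actor whose DoorPanel component slides along its local X axis when opened.
; Every Tick moves the panel's relative location at constant SlideSpeed toward SlideDistance or zero, chosen by the Open flag, without sweeping.
; The OpenDoor event prints a debug string and sets Open to true.
; Nothing in these graphs calls OpenDoor or resets Open to close the door.
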(event Custom|OpenDoor
  (Development|PrintString "DOOR_OPEN_CALLED")
  (Variables|Default|SetbOpen true))

(event EventBeginPlay)

(event Collision|EventActorBeginOverlap
  (params (OtherActor :type Actor%20Object%20Reference)))

(event EventTick
  (params (DeltaSeconds :type Float%20%28single-precision%29))
  (bind _doorpanel (Variables|Default|GetDoorPanel))
  (Transformation|SetRelativeLocation _doorpanel (Math|Interpolation|VInterptoConstant (Variables|/Script/Engine.SceneComponent|GetRelativeLocation _doorpanel) (Math|Vector|MakeVector (Math|Float|SelectFloat (Variables|Default|GetSlideDistance) 0.0 (Variables|Default|GetbOpen)) 0.0 0.0) DeltaSeconds (Variables|Default|GetSlideSpeed)) false false))

(fn ConstructionScript)