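; BP_Door is an interactive door that the player swings open or closed with the F key.
; A box trigger enables input on the door while a BP_ThirdPersonCharacter overlaps it and disables input when it leaves.
; A FlipFlop alternates between playing and reversing a timeline, whose negated track value sets the door component's relative yaw.
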(event OnComponentBeginOverlap(Box)
  (params (OverlappedComponent :type Primitive%20Component%20Object%20Reference) (OtherActor :type Actor%20Object%20Reference) (OtherComp :type Primitive%20Component%20Object%20Reference) (OtherBodyIndex :type Integer) (bFromSweep :type Boolean) (SweepResult :type Hit%20Result%20Structure%20%28by%20ref%29))
  (Utilities|Casting|CastToBP_ThirdPersonCharacter OtherActor)
  (Input|EnableInput (Game|GetPlayerController 0)))

(event OnComponentEndOverlap(Box)
  (params (OverlappedComponent :type Primitive%20Component%20Object%20Reference) (OtherActor :type Actor%20Object%20Reference) (OtherComp :type Primitive%20Component%20Object%20Reference) (OtherBodyIndex :type Integer))
  (Utilities|Casting|CastToBP_ThirdPersonCharacter OtherActor)
  (Input|DisableInput (Game|GetPlayerController 0)))

(event Input|KeyboardEvents|F
  (params (Key :type Key%20Structure :default "None"))
  (:Pressed
    (Utilities|FlowControl|FlipFlop
      (:A
        (bind _新建轨道_0 (Timeline|时间轴 Play)
          (:Update
            (Transformation|SetRelativeRotation (Variables|Default|Get门) (Math|Rotator|MakeRotator 0.0 0.0 (* _新建轨道_0 -1.0)) false false))))
      (:B
        (Timeline|时间轴 Reverse)))))

(fn ConstructionScript)