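; BP_Light is a light that the third-person character switches with the F key.
; Overlapping the sphere enables input and shows a text prompt; leaving hides the prompt but calls EnableInput again, so F keeps working outside the range.
; F drives a FlipFlop that alternately plays and reverses a timeline, which fades the spotlight intensity and hides the prompt while it updates.
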(event OnComponentBeginOverlap(Sphere)
  (params (OverlappedComponent :type Primitive%20Component%20Object%20Reference) (OtherActor :type Actor%20Object%20Reference) (OtherComp :type Primitive%20Component%20Object%20Reference) (OtherBodyIndex :type Integer) (bFromSweep :type Boolean) (SweepResult :type Hit%20Result%20Structure%20%28by%20ref%29))
  (Utilities|Casting|CastToBP_ThirdPersonCharacter OtherActor)
  (Input|EnableInput (Game|GetPlayerController 0))
  (Development|SetHiddeninGame (Variables|Default|GetTextRender) false false))

(event OnComponentEndOverlap(Sphere)
  (params (OverlappedComponent :type Primitive%20Component%20Object%20Reference) (OtherActor :type Actor%20Object%20Reference) (OtherComp :type Primitive%20Component%20Object%20Reference) (OtherBodyIndex :type Integer))
  (Utilities|Casting|CastToBP_ThirdPersonCharacter OtherActor)
  (Input|EnableInput (Game|GetPlayerController 0))
  (Development|SetHiddeninGame (Variables|Default|GetTextRender) true false))

(event Input|KeyboardEvents|F
  (params (Key :type Key%20Structure :default "None"))
  (:Pressed
    (Utilities|FlowControl|FlipFlop
      (:A
        (bind _强度值 (Timeline|时间轴 Play)
          (:Update
            (Rendering|Components|Light|SetIntensity (Variables|Default|GetSpotLight) _强度值)
            (Development|SetHiddeninGame (Variables|Default|GetTextRender) true false))))
      (:B
        (Timeline|时间轴 Reverse)))))

(fn ConstructionScript)