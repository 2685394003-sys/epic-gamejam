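; BP_PowerBox is an interactable power box actor that opens its door and turns on a linked light.
; Pressing F while the player pawn overlaps it sets Opened and unhides the TargetLight actor, with no path to close it again.
; Tick continuously swings DoorMesh toward the open or closed yaw at constant speed, interpolating the rotation's forward vector with VInterpToConstant and converting it back to a rotator.
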(event EventBeginPlay)

(event Collision|EventActorBeginOverlap
  (params (OtherActor :type Actor%20Object%20Reference)))

(event EventTick
  (params (DeltaSeconds :type Float%20%28single-precision%29))
  (bind _doormesh (Variables|Default|GetDoorMesh))
  (Transformation|SetRelativeRotation _doormesh (Math|Conversions|RotationFromXVector (Math|Interpolation|VInterptoConstant (Math|Rotator|GetRotationXVector (Variables|/Script/Engine.SceneComponent|GetRelativeRotation _doormesh)) (Math|Rotator|GetRotationXVector (Math|Rotator|SelectRotator (Math|Rotator|MakeRotator -1.8e+02 0.0 (Variables|Default|GetOpenAngle)) (Math|Rotator|MakeRotator -1.8e+02 0.0 0.0) (Variables|Default|GetbOpened))) DeltaSeconds (Variables|Default|GetSpeed))) false false))

(event Input|KeyboardEvents|F
  (params (Key :type Key%20Structure))
  (:Pressed
    (if (Collision|IsOverlappingActor self (Game|Player|GetPlayerPawn 0) :!class /Script/Engine.Actor)
      (Variables|Default|SetbOpened true)
      (Rendering|SetActorHiddenInGame (Variables|Default|GetTargetLight) false))))

(fn ConstructionScript)