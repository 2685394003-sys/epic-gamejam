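; BP_CardReader is a card reader actor that opens an assigned TargetDoor once it has been powered.
; Activate sets Powered and prints a debug message.
; Tick polls the F key on the first player controller while the player pawn overlaps the reader, then calls OpenDoor if Powered.
; Despite the name, no keycard check is wired; the keycard lookup and other leftover nodes never run.
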(event Custom|Activate
  (Development|PrintString "READER_ACTIVATED" false)
  (Variables|Default|SetbPowered true))

(event EventBeginPlay)

(event Collision|EventActorBeginOverlap
  (params (OtherActor :type Actor%20Object%20Reference)))

(event EventTick
  (params (DeltaSeconds :type Float%20%28single-precision%29))
  (if (and (Game|Player|WasInputKeyJustPressed (Game|GetPlayerController 0) "F") (Collision|IsOverlappingActor self (Game|Player|GetPlayerPawn 0) :!class /Script/Engine.Actor))
    (if (Variables|Default|GetbPowered)
      (Default|OpenDoor (Variables|Default|GetTargetDoor)))))

(fn ConstructionScript)